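; BP_Enemy is a roaming enemy that hunts the player and ends the run by opening the "Muerte" level on reaching them.
; From BeginPlay it moves between random reachable points, pausing after each successful arrival.
; On seeing a pawn, PawnSensing triggers an attack sound and AI movement toward player 0.
; Each sighting also resets a retriggerable delay that sends it back to wandering once it expires.
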(event `self.ReceiveBeginPlay`
  (`self.GoToRandomPoint`))

(event `GoToRandomPoint`
  (`|AIMoveTo` self (`NavigationSystemV1.K2_GetRandomReachablePointInRadius` (`self.K2_GetActorLocation`) 2500.0 null null) null
    (:`OnSuccess`
      (`KismetSystemLibrary.Delay` 3.5)
      (`self.GoToRandomPoint`))))

(event `self.PawnSensing.OnSeePawn`
  (params (Pawn :type "Pawn Object Reference"))
  (`|ExecutionSequence`
    (:`then_0`
      (`|AIMoveTo` self (0.0 0.0 0.0) (`GameplayStatics.GetPlayerPawn` 0)
        (:`then`
          (`GameplayStatics.PlaySound2D` "/Game/Sounds/410326-Monster_Within_-Large_Beast_-Attack-Gen-01.410326-Monster_Within_-Large_Beast_-Attack-Gen-01" 1.0 1.0 0.0 null null))
        (:`OnSuccess`
          (`self.Kill`))))
    (:`then_1`
      (`KismetSystemLibrary.RetriggerableDelay` 3.0)
      (`self.GoToRandomPoint`))))

(event `Kill`
  (`GameplayStatics.OpenLevel` "Muerte"))

(fn `UserConstructionScript`)