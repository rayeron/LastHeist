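; A key-locked door that opens when a first-person character carrying the key (Llave) enters its detection volume.
; Overlapping DoorDetection sets the character's IsInDoor flag, cleared on exit, and calls OpenDoor if the character has the key.
; OpenDoor plays a timeline that drives the yaw of the door cube and two sphere meshes.
; Nothing in the graph closes the door again.
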(event `self.ReceiveBeginPlay`)

(event `OpenDoor`
  (bind (_direction _doorangle) (`Timeline|OpenDoorTL`)
    (:`Update`
      (`SceneComponent.K2_SetRelativeRotation` (`self.museo_Cube_015`) (`KismetMathLibrary.MakeRotator` 0.0 0.0 _doorangle) false false)
      (`SceneComponent.K2_SetRelativeRotation` (`self.museo_Sphere_001`) (`KismetMathLibrary.MakeRotator` 0.0 0.0 _doorangle) false false)
      (`SceneComponent.K2_SetRelativeRotation` (`self.museo_Sphere`) (`KismetMathLibrary.MakeRotator` 0.0 0.0 _doorangle) false false))))

(event `self.DoorDetection.OnComponentBeginOverlap`
  (params (OverlappedComponent :type "PrimitiveComponent Object Reference") (OtherActor :type "Actor Object Reference") (OtherComp :type "PrimitiveComponent Object Reference") (OtherBodyIndex :type Integer) (bFromSweep :type Boolean) (SweepResult :type "HitResult Structure (by ref)"))
  (bind _asbp_first_person_character (cast `/Game/FirstPerson/Blueprints/BP_FirstPersonCharacter` OtherActor))
  (set `/Game/FirstPerson/Blueprints/BP_FirstPersonCharacter.IsInDoor` true _asbp_first_person_character)
  (if (`/Game/FirstPerson/Blueprints/BP_FirstPersonCharacter.Llave` _asbp_first_person_character)
    (`self.OpenDoor`)))

(event `self.DoorDetection.OnComponentEndOverlap`
  (params (OverlappedComponent :type "PrimitiveComponent Object Reference") (OtherActor :type "Actor Object Reference") (OtherComp :type "PrimitiveComponent Object Reference") (OtherBodyIndex :type Integer))
  (bind _asbp_first_person_character (cast `/Game/FirstPerson/Blueprints/BP_FirstPersonCharacter` OtherActor))
  (set `/Game/FirstPerson/Blueprints/BP_FirstPersonCharacter.IsInDoor` false _asbp_first_person_character))

(fn `UserConstructionScript`)